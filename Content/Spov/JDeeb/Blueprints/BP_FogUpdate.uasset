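; BP_FogUpdate is a fog plane that feeds the position of a referenced actor, Mesh, into a flowing fog material.
; The construction script creates a dynamic instance of M_FlowingFog on the Plane component and writes Mesh's root world location to the ActorPos vector parameter.
; Tick rewrites that parameter every frame, so the material tracks the actor as it moves.
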(event EventTick
  (params (DeltaSeconds :type Float%20%28single-precision%29))
  (Rendering|Material|SetVectorParameterValue (Variables|Default|GetDMI) "ActorPos" (Math|Conversions|ToLinearColor(Vector) (Transformation|GetWorldLocation (Variables|/Script/Engine.Actor|GetRootComponent (Variables|Default|GetMesh)))) :!class /Script/Engine.MaterialInstanceDynamic))

(fn ConstructionScript
  (bind _returnvalue (Rendering|Material|CreateDynamicMaterialInstance (Variables|Default|GetPlane) 0 "/Game/Spov/JDeeb/Materials/M_FlowingFog.M_FlowingFog" "None" :!class /Script/Engine.PrimitiveComponent))
  (Variables|Default|SetDMI _returnvalue)
  (Rendering|Material|SetVectorParameterValue (Variables|Default|GetDMI) "ActorPos" (Math|Conversions|ToLinearColor(Vector) (Transformation|GetWorldLocation (Variables|/Script/Engine.Actor|GetRootComponent (Variables|Default|GetMesh)))) :!class /Script/Engine.MaterialInstanceDynamic))