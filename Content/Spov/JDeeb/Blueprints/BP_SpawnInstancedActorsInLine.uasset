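; Construction-script Blueprint that lays out a line of instanced copies of a chosen static mesh.
; It sets the mesh on an InstancedStaticMesh component, then adds GridX instances along local X, spaced by MeshOffset.
; Each instance takes a random yaw from the RandomRots array.
; A matching GridY loop along Y exists but is not connected, and the event graph holds only disabled stubs.
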(event EventBeginPlay)

(event Collision|EventActorBeginOverlap
  (params (OtherActor :type Actor%20Object%20Reference)))

(event EventTick
  (params (DeltaSeconds :type Float%20%28single-precision%29)))

(fn ConstructionScript
  (bind _instancedstaticmesh (Variables|Default|GetInstancedStaticMesh))
  (bind _randomrots (Variables|Default|GetRandomRots))
  (Components|StaticMesh|SetStaticMesh _instancedstaticmesh (Variables|Default|GetStaticMesh))
  (Utilities|FlowControl|Sequence
    (:then_0
      (for _index (range 1 (Variables|Default|GetGridX))
        (Components|InstancedStaticMesh|AddInstance _instancedstaticmesh (Math|Transform|MakeTransform (+ "0, 0, 0" (Math|Vector|MakeVector (* (Variables|Default|GetMeshOffset) (Math|Conversions|ToFloat(Integer) _index)) 0.0 0.0)) (Math|Rotator|MakeRotator 0.0 0.0 (Utilities|Array|Get(acopy) _randomrots (Math|Random|RandomIntegerinRange 0 (- (Utilities|Array|Length _randomrots) 1)))) "1,1,1"))))))