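; BP_InteractiveFog is a configurable volumetric fog actor, built entirely in its construction script.
; It creates a dynamic fog material with box, sphere or texture shapes and hands it to the NSFogWrite Niagara component, sized from the volume.
; For height-based fog, a top-down orthographic scene capture renders selected actors into a float render target that feeds the material.
; The height method can also use actor position, distance fields or none.
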(event EventBeginPlay)

(event Collision|EventActorBeginOverlap
  (params (OtherActor :type Actor%20Object%20Reference)))

(event EventTick
  (params (DeltaSeconds :type Float%20%28single-precision%29)))

(fn ConstructionScript
  (bind _returnvalue (Transformation|GetActorLocation))
  (bind _volumesize (Variables|BaseShape|GetVolumeSize))
  (bind _volumesize_2 (Variables|BaseShape|GetVolumeSize))
  (bind _heightcapture (Variables|Default|GetHeightCapture))
  (bind _ns_fogwrite (Variables|Default|GetNS_FogWrite))
  (bind _returnvalue_2 (Rendering|Material|CreateDynamicMaterialInstance "/Game/Spov/JDeeb/Materials/MaterialInstances/MI_VolumeFog.MI_VolumeFog" "None" "None" :!class /Script/Engine.KismetMaterialLibrary))
  (bind _output_get (Variables|FogSettings|SetFogMID _returnvalue_2))
  (bind _returnvalue_3 (Rendering|CreateRenderTarget2D 256 256 "RTF_R32f"))
  (Variables|FogSettings|SetFogHeightRT _returnvalue_3)
  (Class|NiagaraComponent|SetVariableMaterial (Variables|Default|GetNS_FogWrite) "FogMID" _output_get)
  (Components|Box|SetBoxExtent (Variables|Default|GetDebugBox) (/ (Variables|BaseShape|GetVolumeSize) 2.0) true)
  ;[1 1 1] Dynamically resizing the particle
  (Class|NiagaraComponent|SetVariableMaterial _ns_fogwrite "FogMID" (Variables|FogSettings|GetFogMID))
  (Niagara|SetNiagaraVariable(Float) _ns_fogwrite "VolumeSizeMax" (* (Math|Float|Max(Float) (Math|Float|Max(Float) (.x _volumesize) (.y _volumesize)) (.z _volumesize)) 2.0))
  ;[1 1 1] Shape Settings
  (Rendering|Material|SetVectorParameterValue (Variables|FogSettings|GetFogMID) "ShapeType" (Utilities|Select :Index (Variables|BaseShape|GetShapeType) :NewEnumerator0 "(R=0.000000,G=0.000000,B=1.000000,A=0.000000)" :NewEnumerator1 "(R=0.000000,G=0.000000,B=0.000000,A=1.000000)" :NewEnumerator2 "(R=0.000000,G=1.000000,B=0.000000,A=0.000000)" :NewEnumerator3 "(R=1.000000,G=0.000000,B=0.000000,A=0.000000)") :!class /Script/Engine.MaterialInstanceDynamic)
  (Rendering|Material|SetVectorParameterValue (Variables|FogSettings|GetFogMID) "VolumeSize" (Math|Conversions|ToLinearColor(Vector) (Variables|BaseShape|GetVolumeSize)) :!class /Script/Engine.MaterialInstanceDynamic)
  (Rendering|Material|SetScalarParameterValue (Variables|FogSettings|GetFogMID) "EdgeFalloff" (Variables|BaseShape|GetEdgeFalloff) :!class /Script/Engine.MaterialInstanceDynamic)
  (Rendering|Material|SetTextureParameterValue (Variables|FogSettings|GetFogMID) "Texture2D" (Variables|BaseShape|GetTexture2D))
  (Rendering|Material|SetTextureParameterValue (Variables|FogSettings|GetFogMID) "VolumeTexture" (Variables|BaseShape|GetVolumeTexture))
  (Rendering|Material|SetScalarParameterValue (Variables|FogSettings|GetFogMID) "GlobalExtinction" (Variables|FogSettings|GetGlobalExtinction) :!class /Script/Engine.MaterialInstanceDynamic)
  ;[1 1 1] Height Settings
  (Rendering|Material|SetScalarParameterValue (Variables|FogSettings|GetFogMID) "GlobalHeightFalloff" (Variables|HeightFalloff|GetGlobalHeightFalloff) :!class /Script/Engine.MaterialInstanceDynamic)
  (Rendering|Material|SetTextureParameterValue (Variables|FogSettings|GetFogMID) "HeightRT" (Variables|FogSettings|GetFogHeightRT))
  (Rendering|Material|SetVectorParameterValue (Variables|FogSettings|GetFogMID) "HeightMethod" (Utilities|Select :Index (Variables|HeightFalloff|GetIndex) :NewEnumerator0 "(R=1.000000,G=0.000000,B=0.000000,A=0.000000)" :NewEnumerator1 "(R=0.000000,G=1.000000,B=0.000000,A=0.000000)" :NewEnumerator2 "(R=0.000000,G=0.000000,B=1.000000,A=0.000000)" :NewEnumerator3 "(R=0.000000,G=0.000000,B=0.000000,A=1.000000)") :!class /Script/Engine.MaterialInstanceDynamic)
  ;[1 1 1] HeightCapture
  (Transformation|SetWorldLocationAndRotation _heightcapture (Math|Vector|MakeVector (.x _returnvalue) (.y _returnvalue) (+ (.z _returnvalue) (/ (.z (Variables|BaseShape|GetVolumeSize)) 2.0))) "-90.000000, 0,-90.000000" false false)
  (Variables|/Script/Engine.SceneCaptureComponent2D|SetOrthoWidth _heightcapture (Math|Float|Max(Float) (Math|Float|Max(Float) (.x _volumesize_2) (.y _volumesize_2)) (.z _volumesize_2)))
  (Variables|/Script/Engine.SceneCaptureComponent2D|SetTextureTarget _heightcapture (Variables|FogSettings|GetFogHeightRT))
  (Variables|/Script/Engine.SceneCaptureComponent|SetShowOnlyActors _heightcapture (Variables|HeightFalloff|GetHeightActors))
  (CallFunction|CaptureHeight))

(fn CaptureHeight
  (Rendering|SceneCapture|CaptureScene (Variables|Default|GetHeightCapture) :!class /Script/Engine.SceneCaptureComponent2D)
  (return))