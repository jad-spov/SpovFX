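; Interactive noise fog volume actor that configures a shaped extinction fog effect from its exposed size, color, density and falloff settings.
; The construction script creates a dynamic fog material and passes it to a Niagara fog-write system.
; A top-down orthographic scene capture of chosen actors renders once per construction into a float render target, feeding the material's height falloff.
; One-hot color vectors select shape and height method in the material.
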(event EventBeginPlay)

(event Collision|EventActorBeginOverlap
  (params (OtherActor :type Actor%20Object%20Reference)))

(event EventTick
  (params (DeltaSeconds :type Float%20%28single-precision%29)))

(fn ConstructionScript
  (bind _returnvalue (Rendering|Material|CreateDynamicMaterialInstance "/Game/Spov/JDeeb/Materials/MaterialInstances/MI_ExtinctionFogNoise.MI_ExtinctionFogNoise" "None" "None" :!class /Script/Engine.KismetMaterialLibrary))
  (Variables|Default|SetFogMID _returnvalue)
  (bind _returnvalue_2 (Rendering|CreateRenderTarget2D 256 256 "RTF_R32f"))
  (Variables|Default|SetFogHeightRT _returnvalue_2)
  (Components|Box|SetBoxExtent (Variables|Default|GetDebugBox) (/ (Variables|BaseShape|GetVolumeSize) 2.0) true)
  (CallFunction|SetNiagaraVariables)
  (CallFunction|SetFogMIDVariables)
  (CallFunction|HeightCaptureSetup))

(fn SetNiagaraVariables
  (bind _ns_fogwrite (Variables|Default|GetNS_FogWrite))
  (bind _volumesize (Variables|BaseShape|GetVolumeSize))
  (Class|NiagaraComponent|SetVariableMaterial _ns_fogwrite "FogMID" (Variables|Default|GetFogMID))
  (Niagara|SetNiagaraVariable(Float) _ns_fogwrite "VolumeSizeMax" (* (Math|Float|Max(Float) (Math|Float|Max(Float) (.x _volumesize) (.y _volumesize)) (.z _volumesize)) 2.0))
  (return))

(fn SetFogMIDVariables
  (bind _fogmid (Variables|Default|GetFogMID))
  ;[1 1 1] Base Shape
  (Rendering|Material|SetVectorParameterValue _fogmid "ShapeType" (Utilities|Select :Index (Variables|BaseShape|GetShapeType) :NewEnumerator0 "(R=0.000000,G=0.000000,B=1.000000,A=0.000000)" :NewEnumerator1 "(R=0.000000,G=0.000000,B=0.000000,A=1.000000)" :NewEnumerator2 "(R=0.000000,G=1.000000,B=0.000000,A=0.000000)" :NewEnumerator3 "(R=1.000000,G=0.000000,B=0.000000,A=0.000000)") :!class /Script/Engine.MaterialInstanceDynamic)
  (Rendering|Material|SetVectorParameterValue _fogmid "VolumeSize" (Math|Conversions|ToLinearColor(Vector) (Variables|BaseShape|GetVolumeSize)) :!class /Script/Engine.MaterialInstanceDynamic)
  (Rendering|Material|SetTextureParameterValue _fogmid "Texture2D" (Variables|BaseShape|GetTexture2D))
  (Rendering|Material|SetTextureParameterValue _fogmid "VolumeTexture" (Variables|BaseShape|GetVolumeTexture))
  (Rendering|Material|SetScalarParameterValue _fogmid "EdgeFalloff" (Variables|BaseShape|GetEdgeFalloff) :!class /Script/Engine.MaterialInstanceDynamic)
  ;[1 1 1] Height Falloff
  (Rendering|Material|SetScalarParameterValue _fogmid "GlobalHeightFalloff" (Variables|HeightFalloff|GetGlobalHeightFalloff) :!class /Script/Engine.MaterialInstanceDynamic)
  (Rendering|Material|SetTextureParameterValue _fogmid "HeightRT" (Variables|Default|GetFogHeightRT))
  (Rendering|Material|SetVectorParameterValue _fogmid "HeightMethod" (Utilities|Select :Index (Variables|HeightFalloff|GetHeightMethod) :NewEnumerator4 "(R=1.000000,G=0.000000,B=0.000000,A=0.000000)" :NewEnumerator5 "(R=0.000000,G=1.000000,B=0.000000,A=0.000000)" :NewEnumerator6 "(R=0.000000,G=0.000000,B=1.000000,A=0.000000)" :NewEnumerator7 "(R=0.000000,G=0.000000,B=0.000000,A=1.000000)") :!class /Script/Engine.MaterialInstanceDynamic)
  (Rendering|Material|SetScalarParameterValue _fogmid "GlobalHeightPower" (Variables|HeightFalloff|GetGlobalHeightPower) :!class /Script/Engine.MaterialInstanceDynamic)
  ;[1 1 1] Fog Settings
  (Rendering|Material|SetScalarParameterValue _fogmid "GlobalExtinction" (Variables|FogSettings|GetGlobalExtinction) :!class /Script/Engine.MaterialInstanceDynamic)
  (Rendering|Material|SetVectorParameterValue _fogmid "FogColor" (Variables|FogSettings|GetFogColor) :!class /Script/Engine.MaterialInstanceDynamic)
  (Rendering|Material|SetVectorParameterValue _fogmid "ExtinctionColor" (Variables|FogSettings|GetExtinctionColor) :!class /Script/Engine.MaterialInstanceDynamic)
  (Rendering|Material|SetVectorParameterValue _fogmid "ShadowColor" (Variables|FogSettings|GetShadowColor) :!class /Script/Engine.MaterialInstanceDynamic)
  (Rendering|Material|SetScalarParameterValue _fogmid "ShadowDensity" (Variables|FogSettings|GetShadowDensity) :!class /Script/Engine.MaterialInstanceDynamic)
  (Rendering|Material|SetScalarParameterValue _fogmid "NoiseScale" (Variables|FogSettings|GetNoiseScale) :!class /Script/Engine.MaterialInstanceDynamic)
  (Rendering|Material|SetScalarParameterValue _fogmid "NoisePower" (Variables|FogSettings|GetNoisePower) :!class /Script/Engine.MaterialInstanceDynamic)
  (return))

(fn CaptureHeight
  (Rendering|SceneCapture|CaptureScene (Variables|Default|GetHeightCapture) :!class /Script/Engine.SceneCaptureComponent2D)
  (return))

(fn HeightCaptureSetup
  (bind _returnvalue (Transformation|GetActorLocation))
  (bind _heightcapture (Variables|Default|GetHeightCapture))
  (bind _volumesize (Variables|BaseShape|GetVolumeSize))
  (Transformation|SetWorldLocationAndRotation _heightcapture (Math|Vector|MakeVector (.x _returnvalue) (.y _returnvalue) (+ (.z _returnvalue) (/ (.z (Variables|BaseShape|GetVolumeSize)) 2.0))) "-90.000000, 0,-90.000000" false false)
  (Variables|/Script/Engine.SceneCaptureComponent2D|SetOrthoWidth _heightcapture (Math|Float|Max(Float) (Math|Float|Max(Float) (.x _volumesize) (.y _volumesize)) (.z _volumesize)))
  (Variables|/Script/Engine.SceneCaptureComponent2D|SetTextureTarget _heightcapture (Variables|Default|GetFogHeightRT))
  (Variables|/Script/Engine.SceneCaptureComponent|SetShowOnlyActors _heightcapture (Variables|HeightFalloff|GetHeightActors))
  (HeightFalloff|CaptureHeight))