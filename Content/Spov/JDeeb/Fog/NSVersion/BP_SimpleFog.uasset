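; BP_SimpleFog is a placeable box-shaped fog volume driven by a Niagara system and a fog material.
; Its construction script creates a dynamic instance of MI_SimpleFog_01A and sizes a debug box to the Scale setting.
; It passes that material and a maximum volume size to the NSFogWrite Niagara component.
; Exposed shape, edge and height falloff, color, density and noise settings feed the material; there is no runtime logic.
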(event EventBeginPlay)

(event EventTick
  (params (DeltaSeconds :type Float%20%28single-precision%29)))

(fn ConstructionScript
  (bind _returnvalue (Rendering|Material|CreateDynamicMaterialInstance "/Game/Spov/JDeeb/Fog/NSVersion/MI_SimpleFog_01A.MI_SimpleFog_01A" "None" "None" :!class /Script/Engine.KismetMaterialLibrary))
  (Variables|Default|SetFogMID _returnvalue)
  (Components|Box|SetBoxExtent (Variables|Default|GetDebugBox) (/ (Variables|01-FogShape|GetScale) 2.0) true)
  (CallFunction|SetNiagaraVariables)
  (CallFunction|SetFogMIDVariables))

(fn SetNiagaraVariables
  (bind _ns_fogwrite (Variables|Default|GetNS_FogWrite))
  (bind _scale (Variables|01-FogShape|GetScale))
  (Class|NiagaraComponent|SetVariableMaterial _ns_fogwrite "FogMID" (Variables|Default|GetFogMID))
  (Niagara|SetNiagaraVariable(Float) _ns_fogwrite "VolumeSizeMax" (* (Math|Float|Max(Float) (Math|Float|Max(Float) (.x _scale) (.y _scale)) (.z _scale)) 2.0))
  (return))

(fn SetFogMIDVariables
  (bind _fogmid (Variables|Default|GetFogMID))
  ;[1 1 1] Base Shape
  (Rendering|Material|SetVectorParameterValue _fogmid "VolumeSize" (Math|Conversions|ToLinearColor(Vector) (Variables|01-FogShape|GetScale)) :!class /Script/Engine.MaterialInstanceDynamic)
  (Rendering|Material|SetScalarParameterValue _fogmid "EdgeFalloff" (Variables|01-FogShape|GetEdgeFalloff) :!class /Script/Engine.MaterialInstanceDynamic)
  ;[1 1 1] Height Falloff
  (Rendering|Material|SetScalarParameterValue _fogmid "GlobalHeightFalloff" (Variables|03-FogHeightFalloff|GetHeightFalloff) :!class /Script/Engine.MaterialInstanceDynamic)
  (Rendering|Material|SetScalarParameterValue _fogmid "GlobalHeightPower" (Variables|03-FogHeightFalloff|GetHeightFalloffPower) :!class /Script/Engine.MaterialInstanceDynamic)
  ;[1 1 1] Fog Settings
  (Rendering|Material|SetScalarParameterValue _fogmid "GlobalExtinction" (Variables|00-GlobalSettings|GetGlobalExtinction) :!class /Script/Engine.MaterialInstanceDynamic)
  (Rendering|Material|SetVectorParameterValue _fogmid "FogColor" (Variables|02-FogShading|GetBaseColor) :!class /Script/Engine.MaterialInstanceDynamic)
  (Rendering|Material|SetVectorParameterValue _fogmid "ExtinctionColor" (Variables|02-FogShading|GetTopColor) :!class /Script/Engine.MaterialInstanceDynamic)
  (Rendering|Material|SetVectorParameterValue _fogmid "ShadowColor" (Variables|02-FogShading|GetShadingColor) :!class /Script/Engine.MaterialInstanceDynamic)
  (Rendering|Material|SetScalarParameterValue _fogmid "ShadowDensity" (Variables|02-FogShading|GetDensityShadow) :!class /Script/Engine.MaterialInstanceDynamic)
  (Rendering|Material|SetScalarParameterValue _fogmid "NoiseScale" (Variables|02-FogShading|GetNoiseScaling) :!class /Script/Engine.MaterialInstanceDynamic)
  (Rendering|Material|SetScalarParameterValue _fogmid "NoisePower" (Variables|02-FogShading|GetNoiseStrength) :!class /Script/Engine.MaterialInstanceDynamic)
  (return))