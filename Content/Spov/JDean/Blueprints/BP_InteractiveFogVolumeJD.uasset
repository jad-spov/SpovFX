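; Interactive volumetric fog volume with configurable shape, height falloff, color and noise, rendered through a fog MID handed to the NSFogWrite Niagara system.
; A top-down scene capture records height at construction, while a bottom-up capture records Characters and listed actors each tick.
; An interaction material combines both captures to drive the ripple solver component.
; Solver output is drawn to DebugRT, which feeds both the fog material and a debug plane.
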(event EventBeginPlay
  (bind _outactors (Actor|GetAllActorsOfClass "/Script/Engine.Character"))
  (for _array_element _outactors
    (Rendering|SceneCapture|ShowOnlyActorComponents (Variables|Default|GetInteractionCapture) _array_element false))
  (Default|StartSolver (Variables|Default|GetBPC_RippleSolverComponent)))

(event EventTick
  (params (DeltaSeconds :type Float%20%28single-precision%29))
  (bind _interactionmid (Variables|Default|GetInteractionMID))
  (bind _bpc_ripplesolvercomponent (Variables|Default|GetBPC_RippleSolverComponent))
  (Rendering|SceneCapture|CaptureScene (Variables|Default|GetInteractionCapture) :!class /Script/Engine.SceneCaptureComponent2D)
  (Rendering|DrawMaterialtoRenderTarget (Variables|Default|GetFogInteractionRT) _interactionmid)
  (Default|DrawInteraction _bpc_ripplesolvercomponent _interactionmid)
  ;[1 1 1] Debug Plane
  (Rendering|DrawMaterialtoRenderTarget (Variables|Default|GetDebugRT) (Variables|/Game/Spov/JDeeb/RippleSolver/BPC_RippleSolverComponent.BPC_RippleSolverComponent_C|GetRippleSolverMID _bpc_ripplesolvercomponent)))

(fn ConstructionScript
  (Utilities|FlowControl|Sequence
    (:then_0
      (bind _returnvalue (Rendering|Material|CreateDynamicMaterialInstance "/Game/Spov/JDeeb/Materials/MaterialInstances/MI_VolumeFog.MI_VolumeFog" "None" "None" :!class /Script/Engine.KismetMaterialLibrary))
      (Variables|Default|SetFogMID _returnvalue)
      (bind _returnvalue_2 (Rendering|CreateRenderTarget2D 256 256 "RTF_R32f"))
      (Variables|Default|SetFogHeightCaptureRT _returnvalue_2)
      (bind _returnvalue_3 (Rendering|Material|CreateDynamicMaterialInstance "/Game/Spov/JDeeb/Materials/M_DrawInteraction.M_DrawInteraction" "None" "None" :!class /Script/Engine.KismetMaterialLibrary))
      (Variables|Default|SetInteractionMID _returnvalue_3)
      (bind _returnvalue_4 (Rendering|CreateRenderTarget2D 256 256 "RTF_R32f"))
      (Variables|Default|SetFogInteractionCaptureRT _returnvalue_4)
      (bind _returnvalue_5 (Rendering|CreateRenderTarget2D 256 256 "RTF_R32f"))
      (Variables|Default|SetFogInteractionRT _returnvalue_5)
      (Components|Box|SetBoxExtent (Variables|Default|GetDebugBox) (/ (Variables|01-FogShape|GetScale) 2.0) true)
      (CallFunction|SetNiagaraVariables)
      (CallFunction|SetFogMIDVariables)
      (CallFunction|HeightCaptureSetup)
      (CallFunction|InteractionCaptureSetup)
      (CallFunction|SetInteractionMIDVariables)
      (Default|InitialiseSolver (Variables|Default|GetBPC_RippleSolverComponent)))
    (:then_1
      ;[1 1 1] DebugPlane
      (bind _returnvalue_6 (AddComponent|AddStaticMeshComponent false (Math|Transform|MakeTransform (Math|Vector|MakeVector (.x (Variables|01-FogShape|GetScale)) 0.0 0.0) "90.000000,0.000000, 0" (/ (Variables|01-FogShape|GetScale) 2e+02))))
      (bind _returnvalue_7 (Rendering|Material|CreateDynamicMaterialInstance _returnvalue_6 0 "/Game/Spov/JDeeb/Materials/M_DebugRT.M_DebugRT" "None" :!class /Script/Engine.PrimitiveComponent))
      (bind _output_get (Variables|Default|SetDebugMID _returnvalue_7))
      (bind _returnvalue_8 (Rendering|CreateRenderTarget2D 256 256 "RTF_RGBA16f"))
      (bind _output_get_2 (Variables|Default|SetDebugRT _returnvalue_8))
      (Rendering|Material|SetTextureParameterValue _output_get "DebugRT" _output_get_2)
      (Rendering|Material|SetTextureParameterValue (Variables|Default|GetFogMID) "DebugRT" _output_get_2))))

(fn SetNiagaraVariables
  (bind _ns_fogwrite (Variables|Default|GetNS_FogWrite))
  (bind _scale (Variables|01-FogShape|GetScale))
  (Class|NiagaraComponent|SetVariableMaterial _ns_fogwrite "FogMID" (Variables|Default|GetFogMID))
  (Niagara|SetNiagaraVariable(Float) _ns_fogwrite "VolumeSizeMax" (* (Math|Float|Max(Float) (Math|Float|Max(Float) (.x _scale) (.y _scale)) (.z _scale)) 2.0))
  (return))

(fn SetFogMIDVariables
  (bind _fogmid (Variables|Default|GetFogMID))
  ;[1 1 1] Base Shape
  (Rendering|Material|SetVectorParameterValue _fogmid "ShapeType" (Utilities|Select :Index (Variables|01-FogShape|GetType) :NewEnumerator0 "(R=0.000000,G=0.000000,B=1.000000,A=0.000000)" :NewEnumerator1 "(R=0.000000,G=0.000000,B=0.000000,A=1.000000)" :NewEnumerator2 "(R=0.000000,G=1.000000,B=0.000000,A=0.000000)" :NewEnumerator3 "(R=1.000000,G=0.000000,B=0.000000,A=0.000000)") :!class /Script/Engine.MaterialInstanceDynamic)
  (Rendering|Material|SetVectorParameterValue _fogmid "VolumeSize" (Math|Conversions|ToLinearColor(Vector) (Variables|01-FogShape|GetScale)) :!class /Script/Engine.MaterialInstanceDynamic)
  (Rendering|Material|SetTextureParameterValue _fogmid "Texture2D" (Variables|01-FogShape|Get2DTexture))
  (Rendering|Material|SetTextureParameterValue _fogmid "VolumeTexture" (Variables|01-FogShape|Get3DTexture))
  (Rendering|Material|SetScalarParameterValue _fogmid "EdgeFalloff" (Variables|01-FogShape|GetEdgeFalloff) :!class /Script/Engine.MaterialInstanceDynamic)
  ;[1 1 1] Height Falloff
  (Rendering|Material|SetScalarParameterValue _fogmid "GlobalHeightFalloff" (Variables|03-FogHeightFalloff|GetHeightFalloff) :!class /Script/Engine.MaterialInstanceDynamic)
  (Rendering|Material|SetTextureParameterValue _fogmid "HeightCaptureRT" (Variables|Default|GetFogHeightCaptureRT))
  (Rendering|Material|SetVectorParameterValue _fogmid "HeightMethod" (Utilities|Select :Index (Variables|03-FogHeightFalloff|GetHeightType) :NewEnumerator4 "(R=1.000000,G=0.000000,B=0.000000,A=0.000000)" :NewEnumerator5 "(R=0.000000,G=1.000000,B=0.000000,A=0.000000)" :NewEnumerator6 "(R=0.000000,G=0.000000,B=1.000000,A=0.000000)" :NewEnumerator7 "(R=0.000000,G=0.000000,B=0.000000,A=1.000000)") :!class /Script/Engine.MaterialInstanceDynamic)
  (Rendering|Material|SetScalarParameterValue _fogmid "GlobalHeightPower" (Variables|03-FogHeightFalloff|GetHeightFalloffPower) :!class /Script/Engine.MaterialInstanceDynamic)
  ;[1 1 1] Fog Settings
  (Rendering|Material|SetScalarParameterValue _fogmid "GlobalExtinction" (Variables|00-GlobalSettings|GetGlobalExtinction) :!class /Script/Engine.MaterialInstanceDynamic)
  (Rendering|Material|SetVectorParameterValue _fogmid "FogColor" (Variables|02-FogShading|GetBaseColor) :!class /Script/Engine.MaterialInstanceDynamic)
  (Rendering|Material|SetVectorParameterValue _fogmid "ExtinctionColor" (Variables|02-FogShading|GetTopColor) :!class /Script/Engine.MaterialInstanceDynamic)
  (Rendering|Material|SetVectorParameterValue _fogmid "ShadowColor" (Variables|02-FogShading|GetShadingColor) :!class /Script/Engine.MaterialInstanceDynamic)
  (Rendering|Material|SetScalarParameterValue _fogmid "ShadowDensity" (Variables|02-FogShading|GetDensityShadow) :!class /Script/Engine.MaterialInstanceDynamic)
  (Rendering|Material|SetScalarParameterValue _fogmid "NoiseScale" (Variables|02-FogShading|GetNoiseScaling) :!class /Script/Engine.MaterialInstanceDynamic)
  (Rendering|Material|SetScalarParameterValue _fogmid "NoisePower" (Variables|02-FogShading|GetNoiseStrength) :!class /Script/Engine.MaterialInstanceDynamic)
  (return))

(fn CaptureHeight
  (Rendering|SceneCapture|CaptureScene (Variables|03-FogHeightFalloff|GetHeightCapture) :!class /Script/Engine.SceneCaptureComponent2D)
  (return))

(fn HeightCaptureSetup
  (bind _returnvalue (Transformation|GetActorLocation))
  (bind _heightcapture (Variables|03-FogHeightFalloff|GetHeightCapture))
  (bind _scale (Variables|01-FogShape|GetScale))
  (Transformation|SetWorldLocationAndRotation _heightcapture (Math|Vector|MakeVector (.x _returnvalue) (.y _returnvalue) (+ (.z _returnvalue) (/ (.z (Variables|01-FogShape|GetScale)) 2.0))) "-90.000000, 0,-90.000000" false false)
  (Variables|/Script/Engine.SceneCaptureComponent2D|SetOrthoWidth _heightcapture (Math|Float|Max(Float) (Math|Float|Max(Float) (.x _scale) (.y _scale)) (.z _scale)))
  (Variables|/Script/Engine.SceneCaptureComponent2D|SetTextureTarget _heightcapture (Variables|Default|GetFogHeightCaptureRT))
  (Variables|/Script/Engine.SceneCaptureComponent|SetShowOnlyActors _heightcapture (Variables|03-FogHeightFalloff|GetHeightCaptureActors))
  (HeightFalloff|CaptureHeight))

(fn InteractionCaptureSetup
  (bind _returnvalue (Transformation|GetActorLocation))
  (bind _interactioncapture (Variables|Default|GetInteractionCapture))
  (bind _scale (Variables|01-FogShape|GetScale))
  (Transformation|SetWorldLocationAndRotation _interactioncapture (Math|Vector|MakeVector (.x _returnvalue) (.y _returnvalue) (- (.z _returnvalue) (/ (.z (Variables|01-FogShape|GetScale)) 2.0))) "90.000000,90.000000,180.000000" false false)
  (Variables|/Script/Engine.SceneCaptureComponent2D|SetOrthoWidth _interactioncapture (Math|Float|Max(Float) (Math|Float|Max(Float) (.x _scale) (.y _scale)) (.z _scale)))
  (Variables|/Script/Engine.SceneCaptureComponent2D|SetTextureTarget _interactioncapture (Variables|Default|GetFogInteractionCaptureRT))
  (Variables|/Script/Engine.SceneCaptureComponent|SetShowOnlyActors _interactioncapture (Variables|04-InteractionSettings|GetInteractionCaptureActors))
  (return))

(fn SetInteractionMIDVariables
  (bind _interactionmid (Variables|Default|GetInteractionMID))
  (Rendering|Material|SetTextureParameterValue _interactionmid "InteractionCaptureRT" (Variables|Default|GetFogInteractionCaptureRT))
  (Rendering|Material|SetTextureParameterValue _interactionmid "HeightCaptureRT" (Variables|Default|GetFogHeightCaptureRT))
  (Rendering|Material|SetScalarParameterValue _interactionmid "FogHeight" (Variables|03-FogHeightFalloff|GetHeightFalloff) :!class /Script/Engine.MaterialInstanceDynamic)
  (Rendering|Material|SetScalarParameterValue _interactionmid "Ripple_Pow" (Variables|04-InteractionSettings|GetRipplePower) :!class /Script/Engine.MaterialInstanceDynamic)
  (Rendering|Material|SetScalarParameterValue _interactionmid "None" (Variables|04-InteractionSettings|GetRippleMultiply) :!class /Script/Engine.MaterialInstanceDynamic)
  (return))