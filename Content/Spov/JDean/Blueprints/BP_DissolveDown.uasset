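; BP_DissolveDown plays a dissolve effect on a referenced character's skeletal mesh, on BeginPlay and again whenever the 1 key is pressed.
; It attaches the P_DissolveDown Niagara system and creates a dynamic instance of the mesh's first material, passing both the same texture.
; A timeline drives their shared Amount parameter from one toward zero, keeping material and particles in sync, then zeroes the Niagara Width on finish.
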(event EventBeginPlay
  (bind _character (Variables|Default|GetCharacter))
  (bind _texture (Variables|Default|GetTexture))
  (bind _skeletalmeshcomponent (Variables|/Script/Engine.SkeletalMeshActor|GetSkeletalMeshComponent _character))
  (bind _returnvalue (Niagara|SpawnSystemAttached "/Game/Spov/JDean/Niagara/P_DissolveDown.P_DissolveDown" _skeletalmeshcomponent "None" "0, 0, 0" "0, 0, 0" "KeepRelativeOffset" false))
  (Variables|Default|SetNiagara _returnvalue)
  (bind _returnvalue_2 (Rendering|Material|CreateDynamicMaterialInstance _skeletalmeshcomponent 0 (Rendering|Material|GetMaterial _skeletalmeshcomponent 0) "None" :!class /Script/Engine.PrimitiveComponent))
  (Rendering|Material|SetTextureParameterValue _returnvalue_2 "Texture" _texture)
  (Niagara|SetTextureObject (Variables|Default|GetNiagara) "Texture" _texture)
  (bind _newtrack_0 (Timeline|Timeline_0 PlayFromStart)
    (:Update
      (Rendering|Material|SetScalarParameterValue _returnvalue_2 "Amount" (Math|Float|Lerp 1.0 0.0 _newtrack_0) :!class /Script/Engine.MaterialInstanceDynamic)
      (Niagara|SetNiagaraVariable(Float) (Variables|Default|GetNiagara) "Amount" (Math|Float|Lerp 1.0 0.0 _newtrack_0)))
    (:Finished
      (Niagara|SetNiagaraVariable(Float) (Variables|Default|GetNiagara) "Width" 0.0))))

(event Input|KeyboardEvents|1
  (params (Key :type Key%20Structure :default "None"))
  (bind _character (Variables|Default|GetCharacter))
  (bind _texture (Variables|Default|GetTexture))
  (bind _skeletalmeshcomponent (Variables|/Script/Engine.SkeletalMeshActor|GetSkeletalMeshComponent _character))
  (:Pressed
    (bind _returnvalue (Niagara|SpawnSystemAttached "/Game/Spov/JDean/Niagara/P_DissolveDown.P_DissolveDown" _skeletalmeshcomponent "None" "0, 0, 0" "0, 0, 0" "KeepRelativeOffset" false))
    (Variables|Default|SetNiagara _returnvalue)
    (bind _returnvalue_2 (Rendering|Material|CreateDynamicMaterialInstance _skeletalmeshcomponent 0 (Rendering|Material|GetMaterial _skeletalmeshcomponent 0) "None" :!class /Script/Engine.PrimitiveComponent))
    (Rendering|Material|SetTextureParameterValue _returnvalue_2 "Texture" _texture)
    (Niagara|SetTextureObject (Variables|Default|GetNiagara) "Texture" _texture)
    (bind _newtrack_0 (Timeline|Timeline_0 PlayFromStart)
      (:Update
        (Rendering|Material|SetScalarParameterValue _returnvalue_2 "Amount" (Math|Float|Lerp 1.0 0.0 _newtrack_0) :!class /Script/Engine.MaterialInstanceDynamic)
        (Niagara|SetNiagaraVariable(Float) (Variables|Default|GetNiagara) "Amount" (Math|Float|Lerp 1.0 0.0 _newtrack_0)))
      (:Finished
        (Niagara|SetNiagaraVariable(Float) (Variables|Default|GetNiagara) "Width" 0.0)))))

(fn ConstructionScript)